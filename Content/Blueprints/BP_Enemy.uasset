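; BP_Enemy is an enemy actor that flies in a straight line and explodes on contact with BP_Player.
; At BeginPlay it has a 30% chance to aim at the player's position, otherwise it uses its forward vector.
; Tick moves it along that fixed direction through a Translate helper, without sweep.
; On overlap it spawns an explosion at the player, calls TakeDamage, destroys itself, and destroys the player if that returns true.
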(event `self.ReceiveBeginPlay`
  (if (< (`KismetMathLibrary.RandomFloatInRange` 0.0 1.0) 0.3)
    (bind _returnvalue (`GameplayStatics.GetActorOfClass` "/Game/Blueprints/BP_Player.BP_Player_C"))
    (set `self.Direction` (`KismetMathLibrary.Normal` (- (`self.K2_GetActorLocation` _returnvalue) (`self.K2_GetActorLocation`))))
    (else
      (set `self.Direction` (`self.GetActorForwardVector`)))))

(event `self.ReceiveTick`
  (params (DeltaSeconds :type "Float (single-precision)"))
  (`self.Translate` (`self.Direction`) (`self.Speed`) DeltaSeconds))

(event `self.ReceiveActorBeginOverlap`
  (params (OtherActor :type "Actor Object Reference"))
  ;[1 1 1] 적이 플레이어와 부딪히면 상대의 위치에 폭발VFX를 생성하고 플레이어를 파괴하고 자신도 파괴되고싶다.
  (bind _asbp_player (cast `/Game/Blueprints/BP_Player` OtherActor))
  (`GameplayStatics.SpawnEmitterAtLocation` "/Game/StarterContent/Particles/P_Explosion.P_Explosion" (`self.K2_GetActorLocation` _asbp_player))
  (bind _ishpzero (`/Game/Blueprints/BP_Player.TakeDamage` _asbp_player))
  (if _ishpzero
    (`self.K2_DestroyActor` OtherActor)
    (`self.K2_DestroyActor`)
    (else
      (`self.K2_DestroyActor`))))

(fn `Translate`
  (params (Direction :type "Vector Structure") (Speed :type "Float (double-precision)") (DeltaTime :type "Float (double-precision)"))
  (`self.K2_SetActorLocation` (+ (* (* (`KismetMathLibrary.Normal` Direction) Speed) DeltaTime) (`self.K2_GetActorLocation`))))

(fn `UserConstructionScript`)