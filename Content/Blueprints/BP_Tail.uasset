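; BP_Tail is an actor that chases a target, defaulting to the player.
; BeginPlay fills an unset Target with the BP_Player found in the level.
; Each Tick passes the direction to Target into a Translate helper, which normalizes it and moves the actor by Speed and delta time.
; Movement has no sweep or stopping distance, and Tick does not check that Target is valid.
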(event `self.ReceiveBeginPlay`
  (`/Engine/EditorBlueprintResources/StandardMacros.IsValid` (`self.Target`)
    (:`Is Not Valid`
      ;[1 1 1] 태어날때 BP_Player을 찾아서 Target에 담고싶다.
      (bind _returnvalue (`GameplayStatics.GetActorOfClass` "/Game/Blueprints/BP_Player.BP_Player_C"))
      (`/Engine/EditorBlueprintResources/StandardMacros.IsValid` _returnvalue
        (:`Is Valid`
          (set `self.Target` _returnvalue))))))

(event `self.ReceiveTick`
  (params (DeltaSeconds :type "Float (single-precision)"))
  (`self.Translate` (- (`self.K2_GetActorLocation` (`self.Target`)) (`self.K2_GetActorLocation`)) (`self.Speed`) DeltaSeconds))

(fn `Translate`
  (params (Direction :type "Vector Structure") (Speed :type "Float (double-precision)") (DeltaTime :type "Float (double-precision)"))
  (`self.K2_SetActorLocation` (+ (* (* (`KismetMathLibrary.Normal` Direction) Speed) DeltaTime) (`self.K2_GetActorLocation`))))

(fn `UserConstructionScript`)