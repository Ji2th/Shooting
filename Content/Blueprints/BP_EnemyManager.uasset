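; BP_EnemyManager is an enemy spawner that periodically creates BP_Enemy actors while a BP_Player exists in the level.
; Tick accumulates elapsed time and, once it exceeds CreateTime, spawns an enemy at the Arrow component's world transform regardless of collisions.
; The timer resets only after a spawn, so without a player the lookup repeats every frame until one is found.
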(event `self.ReceiveTick`
  (params (DeltaSeconds :type "Float (single-precision)"))
  ;[1 1 1] 시간이 흐르다가
  ; 현재시간이 생성시간을 초과하면
  ; BP_Enemy를 태어나게하고싶다.
  ; 내가 원하는 위치에 배치하고싶다.
  ; 현재시간을 초기화 하고싶다.
  (bind _output_get (set `self.CurrentTime` (+ DeltaSeconds (`self.CurrentTime`))))
  (if (> _output_get (`self.CreateTime`))
    (bind _returnvalue (`GameplayStatics.GetActorOfClass` "/Game/Blueprints/BP_Player.BP_Player_C"))
    (`/Engine/EditorBlueprintResources/StandardMacros.IsValid` _returnvalue
      (:`Is Valid`
        (`|SpawnActorFromClass` "/Game/Blueprints/BP_Enemy.BP_Enemy_C" (`SceneComponent.K2_GetComponentToWorld` (`self.Arrow`)) "AlwaysSpawn" "OverrideRootScale" null null)
        (set `self.CurrentTime` 0.0)))))

(fn `UserConstructionScript`)