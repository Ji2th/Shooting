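; BP_Bullet is a projectile that flies straight along its forward vector and destroys enemies it hits.
; Tick moves it by Speed times delta time without sweep, so hits rely on overlap events.
; On overlap with a BP_Enemy, it spawns an explosion effect at the enemy's location, then destroys the enemy and itself.
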(event `self.ReceiveActorBeginOverlap`
  (params (OtherActor :type "Actor Object Reference"))
  ;[1 1 1] 총알이 적과 부딪히면 적의 위치에 폭발VFX를 생성하고 적을 파괴하고 자신도 파괴되고싶다.
  (bind _asbp_enemy (cast `/Game/Blueprints/BP_Enemy` OtherActor))
  (`GameplayStatics.SpawnEmitterAtLocation` "/Game/StarterContent/Particles/P_Explosion.P_Explosion" (`self.K2_GetActorLocation` _asbp_enemy))
  (`self.K2_DestroyActor` OtherActor)
  (`self.K2_DestroyActor`))

(event `self.ReceiveTick`
  (params (DeltaSeconds :type "Float (single-precision)"))
  ;[1 1 1] P = P0 + GetActorForward * speed * deltaSeconds
  (`self.K2_SetActorLocation` (+ (`self.K2_GetActorLocation`) (* (* (`self.GetActorForwardVector`) (`self.Speed`)) DeltaSeconds))))

(fn `UserConstructionScript`)