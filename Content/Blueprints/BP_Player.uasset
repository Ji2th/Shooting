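; BP_Player is the player-controlled actor for a shooter, moving in the Y-Z plane and firing from a muzzle point.
; Each Tick passes horizontal and vertical input to a Translate function, which moves it at a normalized, frame-rate-independent speed without collision sweeps.
; The Fire input toggles an auto-fire flag while held.
; Tick uses a Delay to throttle repeated spawns at FirePosition, each followed by a blaster sound.
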(event `self.ReceiveBeginPlay`)

(event `self.ReceiveTick`
  (params (DeltaSeconds :type "Float (single-precision)"))
  (`|ExecutionSequence`
    (:`then_0`
      (`self.Translate` (`KismetMathLibrary.MakeVector` 0.0 (`self.GetInputAxisValue`) (`self.GetInputAxisValue`)) (`self.Speed`) DeltaSeconds))
    (:`then_1`
      (if (`self.IsAutoFire`)
        (`KismetSystemLibrary.Delay` 0.5)
        (`|SpawnActorFromClass` "/Game/Blueprints/BP_Bullet.BP_Bullet_C" (`SceneComponent.K2_GetComponentToWorld` (`self.FirePosition`)) "AlwaysSpawn" "OverrideRootScale" null null)
        (`GameplayStatics.PlaySound2D` "/Game/Audio/star-wars-blaster.star-wars-blaster" 0.2 1.0 0.0 null null)))))

(event `InputAction|Fire`
  (params (Key :type "Key Structure"))
  (:`Pressed`
    (set `self.IsAutoFire` true))
  (:`Released`
    (set `self.IsAutoFire` false)))

(fn `Translate`
  (params (Direction :type "Vector Structure") (Speed :type "Float (double-precision)") (DeltaTime :type "Float (double-precision)"))
  (`self.K2_SetActorLocation` (+ (* (* (`KismetMathLibrary.Normal` Direction) Speed) DeltaTime) (`self.K2_GetActorLocation`))))

(fn `UserConstructionScript`)